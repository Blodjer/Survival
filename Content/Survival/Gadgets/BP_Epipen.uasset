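; BP_Epipen is a Survival gadget that revives another player the user is aiming at.
; On use, it runs a short Pawn object line trace from the owner's camera along the base aim rotation, ignoring the owner.
; A hit SurvivalPlayerCharacter gets Revive called with the Heal value.
; The parent OnUse runs afterward whether or not a player is hit.
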(event EventOnUse
  (bind _ownercharacter (Variables|Default|GetOwnerCharacter))
  (bind _camera (Variables|/Script/Survival.SurvivalPlayerCharacter|GetCamera _ownercharacter))
  (bind _returnvalue (Transformation|GetWorldLocation _camera))
  (bind _outhit (Collision|LineTraceForObjects _returnvalue (+ _returnvalue (* (Math|Vector|GetForwardVector (Pawn|GetBaseAimRotation _ownercharacter)) 5e+02)) (Utilities|Array|MakeArray "ObjectTypeQuery3") false (Utilities|Array|MakeArray _ownercharacter) "None"))
  (bind _assurvival_player_character (Utilities|Casting|CastToSurvivalPlayerCharacter (.HitActor (Collision|BreakHitResult _outhit)))
    (:then
      (Class|SurvivalPlayerCharacter|Revive _assurvival_player_character (Variables|Default|GetHeal)))
    (:CastFailed
      _))
  (|CallParentFunction))

(fn ConstructionScript)