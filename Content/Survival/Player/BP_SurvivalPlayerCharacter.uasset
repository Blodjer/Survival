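; Player character Blueprint for a survival game, handling the local player's UI and cosmetic feedback.
; On local possession it creates UI_Player, removed when view target ends or on destruction.
; Tick drives the flashlight material, switches capsule and EpiPen collision when lethally injured, and feeds health into MPC_Player, post-process deadness effects, hit flashes and speed-scaled camera shake.
; A physics-blend hit reaction exists but is disconnected.
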(event EventOnBecomeViewTarget
  (params (PC :type Player%20Controller%20Object%20Reference)))

(event EventOnEndViewTarget
  (params (PC :type Player%20Controller%20Object%20Reference))
  (if (Pawn|IsLocallyControlled)
    (Utilities|IsValid (stale EventOnPossessedLocal _returnvalue)
      (:Is%20Valid
        (Default|RemoveUserWidget (stale EventOnPossessedLocal _output_get) (stale EventOnPossessedLocal _returnvalue))
        (Widget|RemovefromParent (stale EventOnPossessedLocal _returnvalue))))))

(event Game|Damage|EventPointDamage
  (params (Damage :type Float%20%28single-precision%29) (DamageType :type Damage%20Type%20Object%20Reference) (HitLocation :type Vector :default "0, 0, 0") (HitNormal :type Vector) (HitComponent :type Primitive%20Component%20Object%20Reference) (BoneName :type Name) (ShotFromDirection :type Vector :default "0, 0, 0") (InstigatedBy :type Controller%20Object%20Reference) (DamageCauser :type Actor%20Object%20Reference)))

(event EventUnpossessed
  (params (OldController :type Controller%20Object%20Reference))
  (Rendering|Material|SetScalarParameterValue "/Game/Survival/Player/Materials/MPC_Player.MPC_Player" "Health" 1.0 :!class /Script/Engine.KismetMaterialLibrary)
  (bind _asplayer_controller (Utilities|Casting|CastToPlayerController OldController))
  (Game|Feedback|ClientStopCameraShake _asplayer_controller "/Game/Survival/Player/CameraShakes/BP_MovementForward_CS.BP_MovementForward_CS_C" false))

(event EventTick
  (params (DeltaSeconds :type Float%20%28single-precision%29))
  (bind _returnvalue (Class|SurvivalPlayerCharacter|GetMaxHealth))
  (bind _returnvalue_2 (Class|SurvivalPlayerCharacter|IsLethalInjured))
  (bind _health (Variables|Default|GetHealth))
  (bind _cachedplayercontroller (Variables|Default|GetCachedPlayerController))
  (bind _health_2 (Variables|Default|GetHealth))
  (bind _capsulecomponent (Variables|Default|GetCapsuleComponent))
  (bind _returnvalue_3 (/ _health _returnvalue))
  (Utilities|FlowControl|Sequence
    (:then_0
      (bind _asmaterial_instance_dynamic (Utilities|Casting|CastToMaterialInstanceDynamic (Rendering|Material|GetMaterial (Variables|Character|GetMesh) 1)))
      (Rendering|Material|SetScalarParameterValue _asmaterial_instance_dynamic "Flashlight" (select (Rendering|IsVisible (Variables|Default|GetFlashlight)) (/ (Variables|/Script/Engine.LightComponentBase|GetIntensity (Variables|Default|GetFlashlight)) (Class|SurvivalPlayerCharacter|GetMaxFlashlightIntensity)) 0.0) :!class /Script/Engine.MaterialInstanceDynamic))
    (:then_1
      (Collision|SetCollisionEnabled (Variables|Default|GetEpiPenCollision) (select _returnvalue_2 "QueryOnly" "NoCollision"))
      (Collision|SetCollisionEnabled _capsulecomponent (select _returnvalue_2 "QueryAndPhysics" "QueryOnly"))
      (Collision|SetCollisionResponsetoChannel _capsulecomponent "ECC_Pawn" (select _returnvalue_2 "ECR_Ignore" "ECR_Block")))
    (:then_2
      (if (Pawn|IsLocallyControlled)
        (Utilities|FlowControl|Sequence
          (:then_0
            (bind _returnvalue_4 (Rendering|Material|GetScalarParameterValue "/Game/Survival/Player/Materials/MPC_Player.MPC_Player" "Health" :!class /Script/Engine.KismetMaterialLibrary))
            (Rendering|Material|SetScalarParameterValue "/Game/Survival/Player/Materials/MPC_Player.MPC_Player" "Health" (Math|Interpolation|FInterpTo _returnvalue_4 _returnvalue_3 DeltaSeconds (select (< _returnvalue_4 _returnvalue_3) 0.95 8.5)) :!class /Script/Engine.KismetMaterialLibrary)
            (Utilities|Struct|SetmembersinPostProcessSettings (Variables|/Script/Engine.CameraComponent|GetPostProcessSettings (Variables|Default|GetCamera)) (Class|KismetMathLibrary|LinearColorLerpUsingHSV :A "(R=1.000000,G=1.000000,B=1.000000,A=1.000000)" :Alpha (select (Class|SurvivalPlayerCharacter|IsLethalInjured) (Class|SurvivalPlayerCharacter|GetDeadness) (select (> (Math|Interpolation|FInterpTo _returnvalue_4 _returnvalue_3 DeltaSeconds (select (< _returnvalue_4 _returnvalue_3) 0.95 8.5)) 0.0) 0.0 1.0))) (+ (* (select (Class|SurvivalPlayerCharacter|IsLethalInjured) (Class|SurvivalPlayerCharacter|GetDeadness) (select (> (Math|Interpolation|FInterpTo _returnvalue_4 _returnvalue_3 DeltaSeconds (select (< _returnvalue_4 _returnvalue_3) 0.95 8.5)) 0.0) 0.0 1.0)) 4.5) 0.55) (* (select (Class|SurvivalPlayerCharacter|IsLethalInjured) (Class|SurvivalPlayerCharacter|GetDeadness) (select (> (Math|Interpolation|FInterpTo _returnvalue_4 _returnvalue_3 DeltaSeconds (select (< _returnvalue_4 _returnvalue_3) 0.95 8.5)) 0.0) 0.0 1.0)) 0.3))
            (if (< _health_2 (Variables|Character|GetLastHealth))
              (if (Pawn|IsLocallyControlled)
                (bind _value (Timeline|Timeline_HitFeedback PlayFromStart)
                  (:Update
                    (Rendering|Material|SetScalarParameterValue "/Game/Survival/Player/Materials/MPC_Player.MPC_Player" "HitFeedback" _value :!class /Script/Engine.KismetMaterialLibrary)
                    (Variables|Character|SetLastHealth _health_2 :!label _label))))
              (else
                (goto _label))))
          (:then_1
            (Utilities|IsValid _cachedplayercontroller
              (:Is%20Valid
                (Class|PlayerController|ClientPlayCameraShake _cachedplayercontroller "/Game/Survival/Player/CameraShakes/BP_MovementForward_CS.BP_MovementForward_CS_C" (* (select (AI|Components|NavMovement|IsFalling (Variables|Character|GetCharacterMovement)) 0.0 (/ (Math|Vector|VectorLength (Transformation|GetVelocity)) (Variables|/Script/Survival.SurvivalCharacterMovement|GetMaxWalkSpeedRunning (Variables|Default|GetSurvivalCharacterMovement)))) 0.5) "CameraLocal" "0, 0, 0")))))))))

(event EventOnJumped
  (bind _cachedplayercontroller (Variables|Default|GetCachedPlayerController))
  (Utilities|IsValid _cachedplayercontroller
    (:Is%20Valid
      (Game|Feedback|ClientStopCameraShake _cachedplayercontroller "/Game/Survival/Player/CameraShakes/BP_MovementForward_CS.BP_MovementForward_CS_C" false))))

(event EventDestroyed
  (Utilities|IsValid (stale EventOnPossessedLocal _returnvalue)
    (:Is%20Valid
      (Default|RemoveUserWidget (stale EventOnPossessedLocal _output_get) (stale EventOnPossessedLocal _returnvalue))
      (Widget|RemovefromParent (stale EventOnPossessedLocal _returnvalue)))))

(event EventOnPossessedLocal
  (if (Pawn|IsLocallyControlled)
    (bind _asbp_survival_player_controller (Utilities|Casting|CastToBP_SurvivalPlayerController (Pawn|GetController)))
    (bind _output_get (Variables|Default|SetCachedPlayerController _asbp_survival_player_controller))
    (bind _returnvalue (UserInterface|CreateWidget "/Game/Survival/UI/Player/UI_Player.UI_Player_C" _output_get))
    (UserInterface|Viewport|AddtoPlayerScreen _returnvalue)
    (Default|AddUserWidget _output_get _returnvalue)))

(event EventBeginPlay
  (Variables|Character|SetLastHealth (Class|SurvivalPlayerCharacter|GetMaxHealth)))

(fn ConstructionScript)