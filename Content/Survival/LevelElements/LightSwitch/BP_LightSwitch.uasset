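; BP_LightSwitch is an interactable light switch level element that toggles a set of controlled lights on and off.
; Interact sets the visibility of each ControlledLights light component to the opposite of IsOn, then flips that flag.
; OnRep_IsOn reapplies visibility from IsOn, keeping the lights in sync through replication.
; Interaction queries always report it as usable and rendered as interactable, named "Light Switch" with the verb "Use".
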(event EventInteract
  (params (PlayerCharacter :type Survival%20Player%20Character%20Object%20Reference))
  (for _array_element (Variables|Default|GetControlledLights)
    (Rendering|SetVisibility (Variables|/Script/Engine.Light|GetLightComponent _array_element) (not (Variables|Default|GetIsOn)) false))
  (Variables|Default|SetIsOn (not (Variables|Default|GetIsOn))))

(fn ConstructionScript)

(fn OnRepIson
  (for _array_element (Variables|Default|GetControlledLights)
    (Rendering|SetVisibility (Variables|/Script/Engine.Light|GetLightComponent _array_element) (Variables|Default|GetIsOn) false)))

(fn GetInteractableName
  (return "Light Switch"))

(fn GetInteractionVerb
  (return "Use"))

(fn IsInteractable
  (params (PlayerCharacter :type Survival%20Player%20Character%20Object%20Reference))
  (return true))

(fn IsRenderedasInteractable
  (return true))