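; Time-of-day lighting actor that drives the sun, sky light, sky and celestial spheres, and height fog from the SurvivalGameState clock.
; Each tick SetLighting samples curves by hour, deriving sun rotation and day/night intensity from a TimeShift-remapped time, and feeds dynamic materials and MPC_TimeOfDay.
; Without a game state, it auto-cycles TimeOfDayPreview.
; The construction script applies that preview and can plot the sun's path with instanced meshes.
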(event EventTick
  (params (DeltaSeconds :type Float%20%28single-precision%29))
  (bind _survivalgamestate (Variables|Default|GetSurvivalGameState))
  (Utilities|IsValid _survivalgamestate
    (:Is%20Valid
      (CallFunction|SetLighting (Class|SurvivalGameState|GetTimeOfDay _survivalgamestate)))
    (:Is%20Not%20Valid
      (CallFunction|SetLighting (Math|Float|%(Float) (Variables|Debug|GetTimeOfDayPreview) 24.0))
      (Variables|Debug|SetTimeOfDayPreview (+ (Math|Float|%(Float) (Variables|Debug|GetTimeOfDayPreview) 24.0) (* DeltaSeconds 0.3)))
      (Variables|Clouds|SetCloudSpeed 8.0)
      (Variables|Celestial|SetCelestialSphereSpeed 2.0))))

(event EventBeginPlay
  (bind _assurvival_game_state (Utilities|Casting|CastToSurvivalGameState (Game|GetGameState)))
  (Variables|Default|SetSurvivalGameState _assurvival_game_state))

(fn ConstructionScript
  (bind _returnvalue (Rendering|Material|CreateDynamicMaterialInstance (Variables|Components|GetSkySphere) 0 0 :!class /Script/Engine.PrimitiveComponent))
  (Variables|Sky|SetSkyMaterial _returnvalue)
  (bind _returnvalue_2 (Rendering|Material|CreateDynamicMaterialInstance (Variables|Default|GetCelestialSphere) 0 0 :!class /Script/Engine.PrimitiveComponent))
  (Variables|Celestial|SetCelestialMaterial _returnvalue_2)
  (if (Variables|Debug|GetRefresh)
    _
    (else
      _))
  (Variables|Debug|SetRefresh false)
  (CallFunction|SetLighting (Variables|Debug|GetTimeOfDayPreview))
  (if (Variables|Debug|GetShowSunWay)
    (for _index (range 0 48)
      (Class|InstancedStaticMeshComponent|AddInstanceWorldSpace (Variables|Components|GetInstancedStaticMesh) (Math|Transform|MakeTransform (* (Math|Vector|GetForwardVector (Math|Rotator|MakeRotator (.roll (CallFunction|GetSunRotation (/ (Math|Conversions|ToFloat(Integer) _index) 2.0))) (+ (.pitch (CallFunction|GetSunRotation (/ (Math|Conversions|ToFloat(Integer) _index) 2.0))) 1.8e+02) (.yaw (CallFunction|GetSunRotation (/ (Math|Conversions|ToFloat(Integer) _index) 2.0))))) 1.4e+06) "0, 0, 0" (* "80.000000,80.000000,80.000000" (- 1.0 (Math|Float|%(Float) (/ (Math|Conversions|ToFloat(Integer) _index) 2.0) 1.0))))))))

(fn SetLighting
  (params (TimeOfDay :type Float%20%28single-precision%29))
  (bind _sunlight (Variables|Components|GetSunLight))
  (bind _exponentialheightfog (Variables|Default|GetExponentialHeightFog))
  (bind _skymaterial (Variables|Sky|GetSkyMaterial))
  (bind _skymaterial_2 (Variables|Sky|GetSkyMaterial))
  (bind _skymaterial_3 (Variables|Sky|GetSkyMaterial))
  (bind _celestialmaterial (Variables|Celestial|GetCelestialMaterial))
  (Variables|Time|SetDayNightIntensity (Math|Trig|Sin(Radians) (Math|Float|MultiplybyPi (/ (- (CallFunction|ShiftTimeOfDay TimeOfDay) 6.0) 12.0))))
  (Utilities|FlowControl|Sequence
    (:then_0
      ;[1 1 1] Sun Light
      (Transformation|SetWorldRotation _sunlight (CallFunction|GetSunRotation TimeOfDay) false false)
      (Class|LightComponent|SetTemperature _sunlight (Math|Curves|GetFloatValue (Variables|Sun|GetSunLightTemperature) TimeOfDay))
      (Rendering|Components|Light|SetIntensity _sunlight (* (Math|Float|Clamp(Float) (Math|Trig|Sin(Radians) (/ (Math|Float|MultiplybyPi (Math|Float|MapRangeUnclamped (Variables|Time|GetDayNightIntensity) -0.15 1.0 0.0 1.0)) 2.0))) (Variables|Sun|GetSunLightIntensity)))
      (Rendering|SetVisibility _sunlight (> (* (Math|Float|Clamp(Float) (Math|Trig|Sin(Radians) (/ (Math|Float|MultiplybyPi (Math|Float|MapRangeUnclamped (Variables|Time|GetDayNightIntensity) -0.15 1.0 0.0 1.0)) 2.0))) (Variables|Sun|GetSunLightIntensity)) 0.0) false)
      (Rendering|Material|SetScalarParameterValue "/Game/Survival/TimeOfDay/Materials/MPC_TimeOfDay.MPC_TimeOfDay" "DayNightIntensity" (Math|Float|Clamp(Float) (Math|Trig|Sin(Radians) (/ (Math|Float|MultiplybyPi (Math|Float|MapRangeUnclamped (Variables|Time|GetDayNightIntensity) -0.15 1.0 0.0 1.0)) 2.0))) :!class /Script/Engine.KismetMaterialLibrary))
    (:then_1
      ;[1 1 1] Sky Light
      (Rendering|Components|Light|SetLightColor (Variables|Components|GetSkyLight) (Math|Curves|GetLinearColorValue (Variables|Sky|GetSkyLightColor) TimeOfDay)))
    (:then_2
      ;[1 1 1] Sky Sphere
      (Rendering|Material|SetScalarParameterValue _skymaterial "Time" (Utilities|Time|GetGameTimeinSeconds) :!class /Script/Engine.MaterialInstanceDynamic)
      (Rendering|Material|SetVectorParameterValue _skymaterial "LightDirection" (Math|Conversions|ToLinearColor(Vector) (Math|Rotator|GetRotationXVector (Transformation|GetWorldRotation (Variables|Components|GetSunLight)))) :!class /Script/Engine.MaterialInstanceDynamic)
      (Rendering|Material|SetVectorParameterValue _skymaterial "HorizonColor" (Math|Curves|GetLinearColorValue (Variables|Sky|GetHorizonColor) TimeOfDay) :!class /Script/Engine.MaterialInstanceDynamic)
      (Rendering|Material|SetVectorParameterValue _skymaterial "ZenithColor" (Math|Curves|GetLinearColorValue (Variables|Sky|GetZenithColor) TimeOfDay) :!class /Script/Engine.MaterialInstanceDynamic)
      (Rendering|Material|SetScalarParameterValue _skymaterial "HorizonFalloff" (Math|Float|Lerp 3.5 8.5 (Math|Float|Absolute(Float) (Variables|Time|GetDayNightIntensity))) :!class /Script/Engine.MaterialInstanceDynamic)
      (Rendering|Material|SetScalarParameterValue _skymaterial "DayNightIntensity" (Variables|Time|GetDayNightIntensity) :!class /Script/Engine.MaterialInstanceDynamic)
      (Rendering|Material|SetScalarParameterValue _skymaterial "StarsBrightness" (Variables|Celestial|GetStarsBrightness) :!class /Script/Engine.MaterialInstanceDynamic))
    (:then_3
      ;;[1 1 1] Clouds
      (Rendering|Material|SetVectorParameterValue _skymaterial_3 "CloudColor" (Math|Curves|GetLinearColorValue (Variables|Clouds|GetCloudColor) TimeOfDay) :!class /Script/Engine.MaterialInstanceDynamic)
      (Rendering|Material|SetScalarParameterValue _skymaterial_3 "CloudSpeed" (Variables|Clouds|GetCloudSpeed) :!class /Script/Engine.MaterialInstanceDynamic)
      (Rendering|Material|SetScalarParameterValue _skymaterial_3 "CloudOpacity" (Variables|Clouds|GetCloudOpacity) :!class /Script/Engine.MaterialInstanceDynamic))
    (:then_4
      ;;[1 1 1] Sun
      (Rendering|Material|SetScalarParameterValue _skymaterial_2 "SunRadius" (* (Variables|Sky|GetSunRadius) 0.0003) :!class /Script/Engine.MaterialInstanceDynamic)
      (Rendering|Material|SetScalarParameterValue _skymaterial_2 "SunBrightness" (Variables|Sky|GetSunBrightness) :!class /Script/Engine.MaterialInstanceDynamic)
      (Rendering|Material|SetVectorParameterValue _skymaterial_2 "SunColor" (Variables|Sky|GetSunColor) :!class /Script/Engine.MaterialInstanceDynamic))
    (:then_5
      ;[1 1 1] Celestial
      (Transformation|SetWorldRotation (Variables|Default|GetCelestialSphere) (Math|Rotator|MakeRotator (* (Utilities|Time|GetGameTimeinSeconds) (* (Variables|Celestial|GetCelestialSphereSpeed) -1.0)) (Variables|Celestial|GetLocationLatitude) 0.0) false false)
      (Rendering|Material|SetScalarParameterValue _celestialmaterial "DayNightIntensity" (Variables|Time|GetDayNightIntensity) :!class /Script/Engine.MaterialInstanceDynamic)
      (Rendering|Material|SetScalarParameterValue _celestialmaterial "StarsBrightness" (Variables|Celestial|GetStarsBrightness) :!class /Script/Engine.MaterialInstanceDynamic))
    (:then_6
      ;[1 1 1] Height Fog
      (Class|ExponentialHeightFogComponent|SetFogDensity _exponentialheightfog (Math|Curves|GetFloatValue (Variables|Fog|GetFogDensity) TimeOfDay))
      (Class|ExponentialHeightFogComponent|SetFogInscatteringColor _exponentialheightfog (Math|Curves|GetLinearColorValue (Variables|Fog|GetFogColor) TimeOfDay)))))

(fn GetSunRotation
  (params (TimeOfDay :type Float%20%28single-precision%29))
  (return (Math|Rotator|CombineRotators (Math|Rotator|MakeRotator 0.0 0.0 (+ (Math|Float|Lerp 3.6e+02 0.0 (/ (CallFunction|ShiftTimeOfDay TimeOfDay) 24.0)) 1.8e+02)) (Math|Rotator|MakeRotator 1.8e+02 (* (Variables|Sun|GetSunMaxAltitude) -1.0) 0.0))))

(fn ShiftTimeOfDay
  (params (TimeOfDay :type Float%20%28single-precision%29))
  (return (Math|Curves|GetFloatValue (Variables|Time|GetTimeShift) TimeOfDay)))