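; BP_Door is an interactable housekit door that swings open and closed.
; Interact toggles IsOpen, and Tick rotates DoorMesh at constant Speed toward either OpenDoorAngle yaw or zero.
; The construction script applies StartOpen to both the state and the mesh rotation, so the initial pose shows in the editor.
; It is always interactable, named "Door", with an Open or Close verb that follows its state.
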(event EventInteract
  (params (PlayerCharacter :type Survival%20Player%20Character%20Object%20Reference))
  (Variables|Door|SetIsOpen (not (Variables|Door|GetIsOpen))))

(event EventTick
  (params (DeltaSeconds :type Float%20%28single-precision%29))
  (bind _doormesh (Variables|Default|GetDoorMesh))
  (Transformation|SetRelativeRotation _doormesh (Class|KismetMathLibrary|RInterptoConstant (Variables|/Script/Engine.SceneComponent|GetRelativeRotation _doormesh) (select (Variables|Door|GetIsOpen) (Math|Rotator|MakeRotator 0.0 0.0 (Variables|Door|GetOpenDoorAngle)) "") DeltaSeconds (Variables|Door|GetSpeed)) false false))

(fn ConstructionScript
  (bind _output_get (Variables|Door|SetIsOpen (Variables|Door|GetStartOpen)))
  (Transformation|SetRelativeRotation (Variables|Default|GetDoorMesh) (Math|Rotator|MakeRotator 0.0 0.0 (select _output_get (Variables|Door|GetOpenDoorAngle) 0.0)) false false))

(fn GetInteractableName
  (return "Door"))

(fn GetInteractionVerb
  (return (select (Variables|Door|GetIsOpen) "Close" "Open")))

(fn IsInteractable
  (params (PlayerCharacter :type Survival%20Player%20Character%20Object%20Reference))
  (return true))