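; Sliding barn door that players open and close through interaction, with prompts that follow its current state.
; Interact toggles IsOpen, whose RepNotify restarts the barn door sound.
; Tick slides DoorMesh along local Y at constant speed toward SlideLength or zero, with sweep enabled.
; The construction script applies StartOpen and snaps the mesh to its starting position.
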(event EventInteract
  (params (PlayerCharacter :type Survival%20Player%20Character%20Object%20Reference))
  (Variables|Door|SetIsOpen (not (Variables|Door|GetIsOpen))))

(event EventTick
  (params (DeltaSeconds :type Float%20%28single-precision%29))
  (bind _doormesh (Variables|Default|GetDoorMesh))
  (Transformation|SetRelativeLocation _doormesh (Math|Interpolation|VInterptoConstant (Variables|/Script/Engine.SceneComponent|GetRelativeLocation _doormesh) (Math|Vector|MakeVector 0.0 (select (Variables|Door|GetIsOpen) (Variables|Door|GetSlideLength) 0.0) 0.0) DeltaSeconds (Variables|Door|GetSpeed)) true false))

(fn ConstructionScript
  (bind _output_get (Variables|Door|SetIsOpen (Variables|Door|GetStartOpen)))
  (Transformation|SetRelativeLocation (Variables|Default|GetDoorMesh) (Math|Vector|MakeVector 0.0 (select _output_get (Variables|Door|GetSlideLength) 0.0) 0.0) false false))

(fn OnRepIsOpen
  (bind _audio (Variables|Default|GetAudio))
  (Audio|Components|Audio|Stop _audio)
  (Audio|Components|Audio|SetSound _audio "/Game/Survival/Sound/Environment/SW_DoorBarn.SW_DoorBarn")
  (Audio|Components|Audio|Play _audio 0.0))

(fn GetInteractableName
  (return "Door"))

(fn GetInteractionVerb
  (return (select (Variables|Door|GetIsOpen) "Close" "Open")))

(fn IsInteractable
  (params (PlayerCharacter :type Survival%20Player%20Character%20Object%20Reference))
  (return true))

(fn IsRenderedasInteractable
  (return true))