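; Lighthouse building actor with a rotating spotlight that lights up at night and hides during the day.
; Tick reads time of day from SurvivalGameState, spinning the light during night hours or whenever no valid game state exists.
; Two cross-resetting DoOnce nodes change visibility only on day/night transitions.
; The construction script builds a dynamic Lightbeam material from shape, color, brightness and fade settings, plus a random seed.
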(event EventTick
  (params (DeltaSeconds :type Float%20%28single-precision%29))
  (bind _gamestate (Variables|Default|GetGameState))
  (bind _returnvalue (Class|SurvivalGameState|GetTimeOfDay _gamestate))
  (Utilities|IsValid _gamestate
    (:Is%20Valid
      (if (or (< _returnvalue 7.0) (> _returnvalue 19.5))
        _
        (else
          (Utilities|FlowControl|DoOnce false :!label _label
            (:Completed
              (Rendering|SetVisibility (Variables|Default|GetSpotLight) false true)
              (goto _label_2 Reset))))))
    (:Is%20Not%20Valid
      _))
  (Transformation|AddRelativeRotation (Variables|Default|GetSpotLight) (Math|Rotator|MakeRotator 0.0 0.0 (* DeltaSeconds (Variables|Lighting|GetLightRotationSpeed))) false false)
  (Utilities|FlowControl|DoOnce false :!label _label_2
    (:Completed
      (Rendering|SetVisibility (Variables|Default|GetSpotLight) true true)
      (goto _label Reset))))

(event EventBeginPlay
  (bind _assurvival_game_state (Utilities|Casting|CastToSurvivalGameState (Game|GetGameState))
    (:then
      (Variables|Default|SetGameState _assurvival_game_state))
    (:CastFailed
      (Transformation|AddRelativeRotation (Variables|Default|GetSpotLight) (Math|Rotator|MakeRotator 0.0 0.0 (* (stale EventTick DeltaSeconds) (Variables|Lighting|GetLightRotationSpeed))) false false)
      (Utilities|FlowControl|DoOnce false
        (:Completed
          (Rendering|SetVisibility (Variables|Default|GetSpotLight) true true)
          (Utilities|FlowControl|DoOnce false) ; enters at Reset
        )))))

(fn ConstructionScript
  (bind _returnvalue (Rendering|Material|CreateDynamicMaterialInstance (Variables|Default|GetLightbeam) 0 0 :!class /Script/Engine.PrimitiveComponent))
  (Rendering|Material|SetScalarParameterValue _returnvalue "width" (Variables|Lightbeam|GetWidth) :!class /Script/Engine.MaterialInstanceDynamic)
  (Rendering|Material|SetScalarParameterValue _returnvalue "Length" (Variables|Lightbeam|GetLength) :!class /Script/Engine.MaterialInstanceDynamic)
  (Rendering|Material|SetVectorParameterValue _returnvalue "color" (Variables|Lightbeam|GetColor) :!class /Script/Engine.MaterialInstanceDynamic)
  (Rendering|Material|SetScalarParameterValue _returnvalue "Brightness" (Variables|Lightbeam|GetBrightness) :!class /Script/Engine.MaterialInstanceDynamic)
  (Rendering|Material|SetScalarParameterValue _returnvalue "fadedistance" (Variables|Lightbeam|GetFadeDistance) :!class /Script/Engine.MaterialInstanceDynamic)
  (Rendering|Material|SetScalarParameterValue _returnvalue "random" (Math|Random|RandomFloatinRange 0.0 1e+02) :!class /Script/Engine.MaterialInstanceDynamic))