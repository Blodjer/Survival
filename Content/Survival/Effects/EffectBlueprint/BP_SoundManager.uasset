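; Sound manager that switches forest ambience between night and daytime birds by the time of day in SurvivalGameState.
; Tick polls the time and drives three night forest sounds and one bird sound, with day and night windows slightly overlapping at dawn and dusk.
; DoOnce gates prevent per-frame replays, while random delays stop and re-arm each sound so it restarts periodically.
; Leaving a sound's time window stops it and resets its gate.
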(event EventBeginPlay
  (Audio|Components|Audio|SetSound (Variables|/Script/Engine.AmbientSound|GetAudioComponent (Variables|Default|GetDayBirds1)) "/Game/Survival/Sound/AmbientSound/SW_SoundCueDay1.SW_SoundCueDay1"))

(event EventActorBeginOverlap
  (params (OtherActor :type Actor%20Object%20Reference)))

(event EventTick
  (params (DeltaSeconds :type Float%20%28single-precision%29))
  (bind _nightforrest1 (Variables|Default|GetNightForrest1))
  (bind _nightforrest2 (Variables|Default|GetNightForrest2))
  (bind _nightforrest3 (Variables|Default|GetNightForrest3))
  (bind _daybirds1 (Variables|Default|GetDayBirds1))
  (bind _audiocomponent (Variables|/Script/Engine.AmbientSound|GetAudioComponent _nightforrest1))
  (bind _audiocomponent_2 (Variables|/Script/Engine.AmbientSound|GetAudioComponent _nightforrest2))
  (bind _audiocomponent_3 (Variables|/Script/Engine.AmbientSound|GetAudioComponent _nightforrest3))
  (bind _audiocomponent_4 (Variables|/Script/Engine.AmbientSound|GetAudioComponent _daybirds1))
  (bind _assurvival_game_state (Utilities|Casting|CastToSurvivalGameState (Game|GetGameState)))
  (Utilities|FlowControl|Sequence
    (:then_0
      (if (or (<= (Class|SurvivalGameState|GetTimeOfDay _assurvival_game_state) 5.3) (>= (Class|SurvivalGameState|GetTimeOfDay _assurvival_game_state) 20.8))
        (Utilities|FlowControl|DoOnce false :!label _label
          (:Completed
            (Utilities|FlowControl|Sequence
              (:then_0
                (bind _output_get (Variables|Default|SetSoundNight1 "/Game/Survival/Sound/AmbientSound/SW_NightForrest.SW_NightForrest"))
                (Audio|Components|Audio|SetSound _audiocomponent _output_get)
                (Audio|Components|Audio|Play _audiocomponent 0.0))
              (:then_1
                (Utilities|FlowControl|Delay (Math|Random|RandomFloatinRange 3e+01 5e+01))
                (Audio|Components|Audio|Stop _audiocomponent)
                (goto _label Reset)))))
        (else
          (Variables|Default|SetSoundNight1 0)
          (Audio|Components|Audio|Stop _audiocomponent)
          (goto _label Reset))))
    (:then_1
      (if (or (<= (Class|SurvivalGameState|GetTimeOfDay _assurvival_game_state) 5.3) (>= (Class|SurvivalGameState|GetTimeOfDay _assurvival_game_state) 20.8))
        (Utilities|FlowControl|DoOnce false :!label _label_2
          (:Completed
            (Utilities|FlowControl|Sequence
              (:then_0
                (bind _output_get_2 (Variables|Default|SetSoundNight2 "/Game/Survival/Sound/AmbientSound/SW_NightForrest.SW_NightForrest"))
                (Audio|Components|Audio|SetSound _audiocomponent_2 _output_get_2)
                (Audio|Components|Audio|Play _audiocomponent_2 0.0))
              (:then_1
                (Utilities|FlowControl|Delay (Math|Random|RandomFloatinRange 3e+01 5e+01))
                (Audio|Components|Audio|Stop _audiocomponent_2)
                (goto _label_2 Reset)))))
        (else
          (Variables|Default|SetSoundNight2 0)
          (Audio|Components|Audio|Stop _audiocomponent_2)
          (goto _label_2 Reset))))
    (:then_2
      (if (or (<= (Class|SurvivalGameState|GetTimeOfDay _assurvival_game_state) 5.3) (>= (Class|SurvivalGameState|GetTimeOfDay _assurvival_game_state) 20.8))
        (Utilities|FlowControl|DoOnce false :!label _label_3
          (:Completed
            (Utilities|FlowControl|Sequence
              (:then_0
                (bind _output_get_3 (Variables|Default|SetSoundNight3 "/Game/Survival/Sound/AmbientSound/SW_NightForrest.SW_NightForrest"))
                (Audio|Components|Audio|SetSound _audiocomponent_3 _output_get_3)
                (Audio|Components|Audio|Play _audiocomponent_3 0.0))
              (:then_1
                (Utilities|FlowControl|Delay (Math|Random|RandomFloatinRange 3e+01 5e+01))
                (Audio|Components|Audio|Stop _audiocomponent_3)
                (goto _label_3 Reset)))))
        (else
          (Variables|Default|SetSoundNight3 0)
          (Audio|Components|Audio|Stop _audiocomponent_3)
          (goto _label_3 Reset))))
    (:then_3
      (if (and (>= (Class|SurvivalGameState|GetTimeOfDay _assurvival_game_state) 5.0) (<= (Class|SurvivalGameState|GetTimeOfDay _assurvival_game_state) 21.0))
        (Utilities|FlowControl|Sequence
          (:then_0
            (Utilities|FlowControl|DoOnce false :!label _label_4
              (:Completed
                (Audio|Components|Audio|Play _audiocomponent_4 0.0))))
          (:then_1
            (Utilities|FlowControl|Delay (Math|Random|RandomFloatinRange 3e+01 5e+01))
            (Audio|Components|Audio|Stop _audiocomponent_4)
            (goto _label_4 Reset)))
        (else
          (Audio|Components|Audio|Stop _audiocomponent_4)
          (goto _label_4 Reset))))))

(fn ConstructionScript)