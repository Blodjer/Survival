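; Survival game instance that runs online or LAN session matchmaking and logs each step through colored debug prints.
; StartMatchmaking clears any session and searches, entering the lowest-ping result or creating a session if none is found or entry fails.
; Session creation opens the configured map as a listen server.
; Aborts and travel or network errors destroy the session, whose completion opens MainMenu unless already there.
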(event Custom|Abort%20Matchmaking
  (Debug|DebugLog "Abort Matchmaking...")
  (Debug|DebugLog "Destroy Session...")
  (Class|SurvivalGameInstance|DestroySession))

(event Custom|Start%20Matchmaking
  (params (SessionSettings :type Blueprint%20Session%20Settings%20Structure))
  (Debug|DebugLog "Start Matchmaking...")
  (Class|SurvivalGameInstance|DestroySession)
  (bind _output_get (Variables|Default|SetSessionSettings SessionSettings))
  (Debug|DumpSessionSettings _output_get)
  (Debug|DebugLog "Find Sessions...")
  (Class|SurvivalGameInstance|FindSessions (.islan (Variables|Default|GetSessionSettings)) (.ispresence (Variables|Default|GetSessionSettings)) (.mapname (Variables|Default|GetSessionSettings))))

(event EventFindSessionsComplete
  (params (bWasSuccessful :type Boolean) (SearchResults :type Array%20of%20Blueprint%20Session%20Result%20Structures))
  (bind _sessionsettings (Variables|Default|GetSessionSettings))
  (Debug|DebugSuccess "Find Sessions" bWasSuccessful)
  (if (and bWasSuccessful (> (Utilities|Array|Length SearchResults) 0))
    (bind _index (CallFunction|GetBestSessionResult SearchResults))
    (Debug|DebugLog "Enter Session...")
    (Debug|DumpSessionResult (Utilities|Array|Get(acopy) SearchResults _index))
    (Class|SurvivalGameInstance|EnterSession _index)
    (else
      (Debug|DebugSuccess "No Sessions found" false)
      (Debug|DebugLog "Create Session...")
      (Class|SurvivalGameInstance|CreateSession (.islan _sessionsettings) (.ispresence _sessionsettings) (.mapname _sessionsettings) (.maxnumplayers _sessionsettings)))))

(event EventEnterSessionComplete
  (params (Result :type Integer))
  (bind _returnvalue (== Result 0))
  (bind _sessionsettings (Variables|Default|GetSessionSettings))
  (Debug|DebugSuccess "Enter Sessions Complete" _returnvalue)
  (if (not _returnvalue)
    (Debug|DebugLog "Create Session...")
    (Class|SurvivalGameInstance|CreateSession (.islan _sessionsettings) (.ispresence _sessionsettings) (.mapname _sessionsettings) (.maxnumplayers _sessionsettings))))

(event EventHandleTravelError
  (params (FailureType :type ETravelFailure%20Enum :default "NoLevel"))
  (Debug|DebugSuccess (Utilities|String|EnumtoString FailureType) false)
  (Debug|DebugLog "Destroy Session...")
  (Class|SurvivalGameInstance|DestroySession))

(event EventEndSessionComplete
  (params (bWasSuccessful :type Boolean))
  (Debug|DebugSuccess "End Sessions Complete" bWasSuccessful))

(event EventCreateSessionComplete
  (params (bWasSuccessful :type Boolean))
  (bind _sessionsettings (Variables|Default|GetSessionSettings))
  (bind _returnvalue (Utilities|String|ToString(Integer) (.maxnumplayers _sessionsettings)))
  (bind _returnvalue_2 (select (.islan _sessionsettings) "?bIsLanMatch" ""))
  (bind _returnvalue_3 (Utilities|String|Append "?MaxPlayers=" _returnvalue))
  (bind _returnvalue_4 (Utilities|String|Append "listen" _returnvalue_2 _returnvalue_3))
  (Debug|DebugSuccess "Create Sessions Complete" bWasSuccessful)
  (Debug|DebugLog (Utilities|String|Append "Open Level: " (.mapname _sessionsettings) "?" _returnvalue_4))
  (Game|OpenLevel(byName) (Utilities|String|StringToName (.mapname _sessionsettings)) true _returnvalue_4))

(event EventStartSessionComplete
  (params (bWasSuccessful :type Boolean))
  (Debug|DebugSuccess "Start Sessions Complete" bWasSuccessful))

(event EventDestroySessionComplete
  (params (bWasSuccessful :type Boolean))
  (Debug|DebugSuccess "Destroy Sessions Complete" bWasSuccessful)
  (bind _returnvalue (Game|GetCurrentLevelName true))
  (if (Utilities|Enum|NotEqual(Enum) _returnvalue "MainMenu")
    (Game|OpenLevel(byName) "MainMenu")))

(event EventHandleNetworkError
  (params (FailureType :type ENetworkFailure%20Enum :default "NetDriverAlreadyExists") (bIsServer :type Boolean))
  (Debug|DebugSuccess (Utilities|String|EnumtoString FailureType) false)
  (Debug|DebugLog "Destroy Session...")
  (Class|SurvivalGameInstance|DestroySession))

(event EventInit
  (bind _returnvalue (Class|SurvivalGameInstance|IsOnlineSubystemReady))
  (if (not _returnvalue)
    (Debug|DebugSuccess "Online Subsystem not found" _returnvalue)))

(fn DebugLog
  (params (Log :type String))
  (Development|PrintString Log true true "(R=0.000000,G=0.660000,B=1.000000,A=1.000000)" (Variables|Debug|GetDebugLogDuration)))

(fn DebugSuccess
  (params (Log :type String) (Success :type Boolean))
  (Development|PrintString (Utilities|String|Append (select Success "Success" "Failure") ": " Log) true true (select Success "(R=0.000000,G=1.000000,B=0.000000,A=1.000000)" "(R=1.000000,G=0.000000,B=0.000000,A=1.000000)") (Variables|Debug|GetDebugLogDuration)))

(fn GetBestSessionResult
  (params (SearchResults :type Array%20of%20Blueprint%20Session%20Result%20Structures))
  (for (_array_element _array_index) SearchResults
    (if (< (Class|FindSessionsCallbackProxy|GetPinginMs _array_element) (Class|FindSessionsCallbackProxy|GetPinginMs (Utilities|Array|Get(acopy) SearchResults (LocalVariables|GetCurrentBestResult))))
      (LocalVariables|SetCurrentBestResult _array_index)))
  (return (LocalVariables|GetCurrentBestResult)))

(fn DumpSessionSettings
  (params (SessionSettings :type Blueprint%20Session%20Settings%20Structure))
  (bind _returnvalue (Utilities|String|ToString(Boolean) (.islan SessionSettings)))
  (bind _returnvalue_2 (Utilities|String|ToString(Integer) (.maxnumplayers SessionSettings)))
  (bind _returnvalue_3 (Utilities|String|ToString(Boolean) (.ispresence SessionSettings)))
  (bind _returnvalue_4 (Utilities|String|Append "Map:  " (.mapname SessionSettings)))
  (bind _returnvalue_5 (Utilities|String|Append "Presence:  " _returnvalue_3))
  (bind _returnvalue_6 (Utilities|String|Append "Players:  " _returnvalue_2))
  (bind _returnvalue_7 (Utilities|String|Append "Local:  " _returnvalue))
  (bind _array (Utilities|Array|MakeArray "Dump Matchmaking Settings..." _returnvalue_4 _returnvalue_6 _returnvalue_7 _returnvalue_5))
  (bind _returnvalue_8 (Utilities|Array|Length _array))
  (for _index (range 1 _returnvalue_8)
    (Development|PrintString (Utilities|Array|Get(acopy) _array (- _returnvalue_8 _index)) true false "(R=0.720000,G=0.252000,B=0.657599,A=1.000000)" (Variables|Debug|GetDebugLogDuration))
    (Development|PrintString (Utilities|Array|Get(acopy) _array (- _index 1)) false true "(R=0.720000,G=0.252000,B=0.657599,A=1.000000)" (Variables|Debug|GetDebugLogDuration))))

(fn DumpSessionResult
  (params (SessionResult :type Blueprint%20Session%20Result%20Structure))
  (bind _returnvalue (Class|FindSessionsCallbackProxy|GetCurrentPlayers SessionResult))
  (bind _returnvalue_2 (Class|FindSessionsCallbackProxy|GetMaxPlayers SessionResult))
  (bind _returnvalue_3 (Class|FindSessionsCallbackProxy|GetPinginMs SessionResult))
  (bind _returnvalue_4 (Class|FindSessionsCallbackProxy|GetServerName SessionResult))
  (bind _returnvalue_5 (Utilities|String|ToString(Integer) _returnvalue))
  (bind _returnvalue_6 (Utilities|String|ToString(Integer) _returnvalue_3))
  (bind _returnvalue_7 (Utilities|String|ToString(Integer) _returnvalue_2))
  (bind _returnvalue_8 (Utilities|String|Append "ServerName:  " _returnvalue_4))
  (bind _returnvalue_9 (Utilities|String|Append "MaxPlayers:  " _returnvalue_7))
  (bind _returnvalue_10 (Utilities|String|Append "CurrentPlayers:  " _returnvalue_5))
  (bind _returnvalue_11 (Utilities|String|Append "Ping:  " _returnvalue_6))
  (bind _array (Utilities|Array|MakeArray "Dump Matchmaking Settings..." _returnvalue_8 _returnvalue_10 _returnvalue_9 _returnvalue_11))
  (bind _returnvalue_12 (Utilities|Array|Length _array))
  (for _index (range 1 _returnvalue_12)
    (Development|PrintString (Utilities|Array|Get(acopy) _array (- _returnvalue_12 _index)) true false "(R=0.720000,G=0.252000,B=0.657599,A=1.000000)" (Variables|Debug|GetDebugLogDuration))
    (Development|PrintString (Utilities|Array|Get(acopy) _array (- _index 1)) false true "(R=0.720000,G=0.252000,B=0.657599,A=1.000000)" (Variables|Debug|GetDebugLogDuration))))