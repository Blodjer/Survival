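; Save game object for the survival game's graphics settings, covering scalability qualities, motion blur and frame rate cap.
; SetGraphicSetting stores a value by setting type, then returns a string joining the matching console variable name and value, with motion blur scaled from percent to a fraction.
; It only builds that string and does not execute it.
; GetGraphicSetting returns the stored value for a given setting type.
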(fn SetGraphicSetting
  (params (Setting :type EGraphicSettings%20Enum) (Value :type Integer))
  (bind _returnvalue (Utilities|String|ToString(Integer) Value))
  (Utilities|FlowControl|Sequence
    (:then_0
      (switch Utilities|FlowControl|Switch|SwitchonEGraphicSettings Setting
        (:NewEnumerator0
          (Variables|Default|SetTextureQuality Value))
        (:NewEnumerator1
          (Variables|Default|SetShadowQuality Value))
        (:NewEnumerator2
          (Variables|Default|SetFoliageDensity Value))
        (:NewEnumerator3
          (Variables|Default|SetAntiAliasingQuality Value))
        (:NewEnumerator4
          (Variables|Default|SetEffectsQuality Value))
        (:NewEnumerator5
          (Variables|Default|SetViewDistance Value))
        (:NewEnumerator6
          (Variables|Default|SetPostProcessingQuality Value))
        (:NewEnumerator8
          (Variables|Default|SetMotionBlur Value))
        (:NewEnumerator7
          (Variables|Default|SetFramerate Value))))
    (:then_1
      (return (Utilities|String|Append (Utilities|Select :Index Setting :NewEnumerator0 "sg.TextureQuality" :NewEnumerator1 "sg.ShadowQuality" :NewEnumerator2 "sg.FoliageQuality" :NewEnumerator3 "sg.AntiAliasingQuality" :NewEnumerator4 "sg.EffectsQuality" :NewEnumerator5 "sg.ViewDistanceQuality" :NewEnumerator6 "sg.PostProcessQuality" :NewEnumerator8 "r.MotionBlur.Amount" :NewEnumerator7 "t.MaxFPS") " " (Utilities|Select :Index Setting :NewEnumerator0 _returnvalue :NewEnumerator1 _returnvalue :NewEnumerator2 _returnvalue :NewEnumerator3 _returnvalue :NewEnumerator4 _returnvalue :NewEnumerator5 _returnvalue :NewEnumerator6 _returnvalue :NewEnumerator8 (Utilities|String|ToString(Float) (/ (Math|Conversions|ToFloat(Integer) Value) 1e+02)) :NewEnumerator7 _returnvalue))))))

(fn GetGraphicSetting
  (params (Setting :type EGraphicSettings%20Enum))
  (return (Utilities|Select :Index Setting :NewEnumerator0 (Variables|Default|GetTextureQuality) :NewEnumerator1 (Variables|Default|GetShadowQuality) :NewEnumerator2 (Variables|Default|GetFoliageDensity) :NewEnumerator3 (Variables|Default|GetAntiAliasingQuality) :NewEnumerator4 (Variables|Default|GetEffectsQuality) :NewEnumerator5 (Variables|Default|GetViewDistance) :NewEnumerator6 (Variables|Default|GetPostProcessingQuality) :NewEnumerator8 (Variables|Default|GetMotionBlur) :NewEnumerator7 (Variables|Default|GetFramerate))))