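; Blueprint function library that reads, saves and applies the game's graphic settings through the SurvivalSettings save slot.
; SetGraphicSetting loads the save object, has it store a value, runs the console command it returns, then saves the slot.
; GetGraphicSetting returns the saved value, or 0 when no valid save exists.
; ApplyAllSettings loops over every graphic setting enum entry, feeding each saved value back through SetGraphicSetting.
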(fn SetGraphicSetting
  (params (Setting :type EGraphicSettings%20Enum) (Value :type Integer))
  (bind _returnvalue (SaveGame|LoadGamefromSlot "SurvivalSettings"))
  (bind _assurvival_save_game_settings (Utilities|Casting|CastToSurvivalSaveGameSettings _returnvalue))
  (bind _consolecommand (Default|SetGraphicSetting _assurvival_save_game_settings Setting Value))
  (Development|ExecuteConsoleCommand 0 _consolecommand)
  (SaveGame|SaveGametoSlot _assurvival_save_game_settings "SurvivalSettings"))

(fn GetGraphicSetting
  (params (Setting :type EGraphicSettings%20Enum))
  (bind _returnvalue (SaveGame|DoesSaveGameExist "SurvivalSettings"))
  (if _returnvalue
    (bind _returnvalue_2 (SaveGame|LoadGamefromSlot "SurvivalSettings"))
    (bind _assurvival_save_game_settings (Utilities|Casting|CastToSurvivalSaveGameSettings _returnvalue_2)
      (:then
        (bind _value (Default|GetGraphicSetting _assurvival_save_game_settings Setting))
        (return _value))
      (:CastFailed
        _)))
  (return 0))

(fn ApplyAllSettings
  (bind _enumvalue (|ForEachEGraphicSettings)
    (:LoopBody
      (bind _value (CallFunction|GetGraphicSetting _enumvalue))
      (CallFunction|SetGraphicSetting _enumvalue _value))))