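; Survival-mode player controller that manages the local player's UI through match waiting, countdown, death and respawn, winner screen and pause menu.
; Match and life events create or remove widgets, with a gate that blocks the respawn screen once the match ends.
; Most widgets register in a shared list so the pause menu or H key can hide them together.
; Tick rebuilds teammate markers, kept outside that list, whenever the spawned teammate count changes.
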(event EventOnDeath
  (Utilities|FlowControl|Gate false
    (:Exit
      (if (Pawn|IsLocalController)
        (bind _returnvalue (UserInterface|CreateWidget "/Game/Survival/UI/Player/UI_Respawn.UI_Respawn_C" self))
        (UserInterface|Viewport|AddtoPlayerScreen _returnvalue)
        (CallFunction|AddUserWidget _returnvalue)))))

(event EventTick
  (params (DeltaSeconds :type Float%20%28single-precision%29))
  (bind _playermarkerwidgets (Variables|UserInterface|GetPlayerMarkerWidgets))
  (if (Pawn|IsLocalPlayerController)
    (Utilities|FlowControl|Sequence
      (:then_0
        (bind _assurvival_player_state (Utilities|Casting|CastToSurvivalPlayerState (Variables|Default|GetPlayerState)))
        (bind _returnvalue (Class|SurvivalPlayerState|GetSpawnedTeamMates _assurvival_player_state))
        (if (!= (Utilities|Array|Length _returnvalue) (Variables|UserInterface|GetSpawnedTeamMates))
          (for _array_element _playermarkerwidgets
            (Widget|RemovefromParent _array_element))
          (Utilities|Array|Clear _playermarkerwidgets)
          (for _array_element_2 _returnvalue
            (bind _returnvalue_2 (UserInterface|CreateWidget "/Game/Survival/UI/Prefabs/UI_PlayerMarker.UI_PlayerMarker_C" self _array_element_2))
            (UserInterface|Viewport|AddtoPlayerScreen _returnvalue_2)
            (Class|UserWidget|SetDesiredSizeinViewport _returnvalue_2 "(X=400.000000,Y=200.000000)")
            (Utilities|Array|Add (Variables|UserInterface|GetPlayerMarkerWidgets) _returnvalue_2))
          (Variables|UserInterface|SetSpawnedTeamMates (Utilities|Array|Length _returnvalue)))))))

(event EventBeginPlay
  (if (Pawn|IsLocalController)
    (bind _returnvalue (UserInterface|CreateWidget "/Game/Survival/UI/Player/UI_Environment.UI_Environment_C" self))
    (UserInterface|Viewport|AddtoViewport _returnvalue 0)
    (CallFunction|AddUserWidget _returnvalue)))

(event EventOnMatchHasStarted
  (Utilities|IsValid (stale EventOnMatchHasStartedCountdown _returnvalue)
    (:Is%20Valid
      (CallFunction|RemoveUserWidget (stale EventOnMatchHasStartedCountdown _returnvalue))
      (Widget|RemovefromParent (stale EventOnMatchHasStartedCountdown _returnvalue)))
    (:Is%20Not%20Valid
      _))
  (Utilities|IsValid (stale EventOnMatchIsWaitingforPlayers _returnvalue)
    (:Is%20Valid
      (CallFunction|RemoveUserWidget (stale EventOnMatchIsWaitingforPlayers _returnvalue))
      (Widget|RemovefromParent (stale EventOnMatchIsWaitingforPlayers _returnvalue)))))

(event EventOnMatchHasEnded
  (params (WinnerTeamIdx :type Integer))
  (if (>= WinnerTeamIdx 0)
    (bind _assurvival_game_state (Utilities|Casting|CastToSurvivalGameState (Game|GetGameState)))
    (bind _returnvalue (Class|SurvivalGameState|GetTeamInfo _assurvival_game_state WinnerTeamIdx))
    (bind _returnvalue_2 (UserInterface|CreateWidget "/Game/Survival/UI/Match/UI_PresentWinner.UI_PresentWinner_C" self _returnvalue))
    (UserInterface|Viewport|AddtoViewport _returnvalue_2 0)
    (CallFunction|AddUserWidget _returnvalue_2))
  (Utilities|FlowControl|Sequence
    (:then_0
      (Utilities|FlowControl|Gate false) ; enters at Close
    )
    (:then_1
      (Utilities|IsValid (stale EventOnDeath _returnvalue)
        (:Is%20Valid
          (CallFunction|RemoveUserWidget (stale EventOnDeath _returnvalue))
          (Widget|RemovefromParent (stale EventOnDeath _returnvalue)))))))

(event EventOnRespawn
  (Utilities|IsValid (stale EventOnDeath _returnvalue)
    (:Is%20Valid
      (CallFunction|RemoveUserWidget (stale EventOnDeath _returnvalue))
      (Widget|RemovefromParent (stale EventOnDeath _returnvalue)))))

(event EventOnMatchIsWaitingforPlayers
  (bind _returnvalue (UserInterface|CreateWidget "/Game/Survival/UI/Match/UI_WaitingForPlayers.UI_WaitingForPlayers_C" self))
  (UserInterface|Viewport|AddtoViewport _returnvalue 0)
  (CallFunction|AddUserWidget _returnvalue))

(event EventOnOpenPauseMenu
  (bind _returnvalue (UserInterface|CreateWidget "/Game/Survival/UI/InGameMenu/UI_InGameMenu.UI_InGameMenu_C" self))
  (UserInterface|Viewport|AddtoViewport _returnvalue 50)
  (CallFunction|SetHudVisible false))

(event EventOnClosePauseMenu
  (Utilities|IsValid (stale EventOnOpenPauseMenu _returnvalue)
    (:Is%20Valid
      (Widget|RemovefromParent (stale EventOnOpenPauseMenu _returnvalue)))
    (:Is%20Not%20Valid
      _))
  (CallFunction|SetHudVisible true))

(event EventOnMatchHasStartedCountdown
  (params (RemainingTime :type Float%20%28single-precision%29))
  (bind _returnvalue (UserInterface|CreateWidget "/Game/Survival/UI/Match/UI_MatchStartCountdown.UI_MatchStartCountdown_C" self RemainingTime))
  (UserInterface|Viewport|AddtoViewport _returnvalue 0)
  (CallFunction|AddUserWidget _returnvalue)
  (Utilities|IsValid (stale EventOnMatchIsWaitingforPlayers _returnvalue)
    (:Is%20Valid
      (CallFunction|RemoveUserWidget (stale EventOnMatchIsWaitingforPlayers _returnvalue))
      (Widget|RemovefromParent (stale EventOnMatchIsWaitingforPlayers _returnvalue)))))

(event Input|KeyboardEvents|H
  (params (Key :type Key%20Structure :default "AnyKey"))
  ;[1 1 1] Dirty
  (:Pressed
    (Utilities|IsValid (stale EventOnOpenPauseMenu _returnvalue)
      (:Is%20Not%20Valid
        (CallFunction|SetHudVisible (not (Variables|UserInterface|GetIsUserWidgetsVisible)))))))

(fn ConstructionScript)

(fn AddUserWidget
  (params (Widget :type User%20Widget%20Object%20Reference%20%28by%20ref%29))
  (Utilities|Array|Add (Variables|UserInterface|GetUserWidgets) Widget)
  (Widget|SetVisibility Widget (select (Variables|UserInterface|GetIsUserWidgetsVisible) "HitTestInvisible" "Hidden")))

(fn RemoveUserWidget
  (params (Widget :type User%20Widget%20Object%20Reference))
  (Utilities|Array|RemoveItem (Variables|UserInterface|GetUserWidgets) Widget))

(fn SetHudVisible
  (params (Visible :type Boolean))
  (for _array_element (Variables|UserInterface|GetUserWidgets)
    (Widget|SetVisibility _array_element (select Visible "HitTestInvisible" "Hidden")))
  (Variables|UserInterface|SetIsUserWidgetsVisible Visible))