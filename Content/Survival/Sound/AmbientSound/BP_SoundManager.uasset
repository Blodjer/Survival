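; Ambient sound manager that switches forest and "Berg" audio between day and night sets based on the survival game state's time of day.
; BeginPlay caches the game state and calls SetSound on each audio component.
; Every Tick, separate branches play each in-window sound once via DoOnce, then stop and re-arm it after a random delay.
; Out-of-window sounds stop immediately, and the two windows overlap slightly at dawn and dusk.
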(event EventBeginPlay
  (Utilities|FlowControl|Sequence
    (:then_0
      (bind _assurvival_game_state (Utilities|Casting|CastToSurvivalGameState (Game|GetGameState)))
      (Variables|Default|SetSurvivalGameState _assurvival_game_state))
    (:then_1
      (Utilities|FlowControl|Sequence
        (:then_0
          (Audio|Components|Audio|SetSound (Variables|/Script/Engine.AmbientSound|GetAudioComponent (Variables|Default|GetDay1Berg)) 0)
          (Audio|Components|Audio|SetSound (Variables|/Script/Engine.AmbientSound|GetAudioComponent (Variables|Default|GetNightBerg)) 0))
        (:then_1
          (Audio|Components|Audio|SetSound (Variables|/Script/Engine.AmbientSound|GetAudioComponent (Variables|Default|GetDay1)) 0)
          (Audio|Components|Audio|SetSound (Variables|/Script/Engine.AmbientSound|GetAudioComponent (Variables|Default|GetNightForrest1)) 0))
        (:then_2
          (Audio|Components|Audio|SetSound (Variables|/Script/Engine.AmbientSound|GetAudioComponent (Variables|Default|GetDay2)) 0)
          (Audio|Components|Audio|SetSound (Variables|/Script/Engine.AmbientSound|GetAudioComponent (Variables|Default|GetNightForrest2)) 0))
        (:then_3
          (Audio|Components|Audio|SetSound (Variables|/Script/Engine.AmbientSound|GetAudioComponent (Variables|Default|GetDay3)) 0)
          (Audio|Components|Audio|SetSound (Variables|/Script/Engine.AmbientSound|GetAudioComponent (Variables|Default|GetNightForrest3)) 0))
        (:then_4
          (Audio|Components|Audio|SetSound (Variables|/Script/Engine.AmbientSound|GetAudioComponent (Variables|Default|GetDay4)) 0))))))

(event EventTick
  (params (DeltaSeconds :type Float%20%28single-precision%29))
  (bind _nightberg (Variables|Default|GetNightBerg))
  (bind _nightforrest1 (Variables|Default|GetNightForrest1))
  (bind _nightforrest2 (Variables|Default|GetNightForrest2))
  (bind _nightforrest3 (Variables|Default|GetNightForrest3))
  (bind _day1berg (Variables|Default|GetDay1Berg))
  (bind _day1 (Variables|Default|GetDay1))
  (bind _day2 (Variables|Default|GetDay2))
  (bind _day3 (Variables|Default|GetDay3))
  (bind _day4 (Variables|Default|GetDay4))
  (bind _survivalgamestate (Variables|Default|GetSurvivalGameState))
  (bind _returnvalue (Class|SurvivalGameState|GetTimeOfDay _survivalgamestate))
  (bind _audiocomponent (Variables|/Script/Engine.AmbientSound|GetAudioComponent _nightberg))
  (bind _audiocomponent_2 (Variables|/Script/Engine.AmbientSound|GetAudioComponent _nightforrest1))
  (bind _audiocomponent_3 (Variables|/Script/Engine.AmbientSound|GetAudioComponent _nightforrest2))
  (bind _audiocomponent_4 (Variables|/Script/Engine.AmbientSound|GetAudioComponent _nightforrest3))
  (bind _audiocomponent_5 (Variables|/Script/Engine.AmbientSound|GetAudioComponent _day1berg))
  (bind _audiocomponent_6 (Variables|/Script/Engine.AmbientSound|GetAudioComponent _day1))
  (bind _audiocomponent_7 (Variables|/Script/Engine.AmbientSound|GetAudioComponent _day2))
  (bind _audiocomponent_8 (Variables|/Script/Engine.AmbientSound|GetAudioComponent _day3))
  (bind _audiocomponent_9 (Variables|/Script/Engine.AmbientSound|GetAudioComponent _day4))
  (Utilities|FlowControl|Sequence
    (:then_0
      ;[1 1 1] Night1
      (if (or (<= _returnvalue 5.3) (>= _returnvalue 20.8))
        (Utilities|FlowControl|Sequence
          (:then_0
            (Utilities|FlowControl|DoOnce false :!label _label
              (:Completed
                (Audio|Components|Audio|Play _audiocomponent_2 0.0))))
          (:then_1
            (Utilities|FlowControl|Delay (Math|Random|RandomFloatinRange 3e+01 5e+01))
            (Audio|Components|Audio|Stop _audiocomponent_2)
            (goto _label Reset)))
        (else
          (Audio|Components|Audio|Stop _audiocomponent_2)
          (goto _label Reset))))
    (:then_1
      ;[1 1 1] Night2
      (if (or (<= _returnvalue 5.3) (>= _returnvalue 20.8))
        (Utilities|FlowControl|Sequence
          (:then_0
            (Utilities|FlowControl|DoOnce false :!label _label_2
              (:Completed
                (Audio|Components|Audio|Play _audiocomponent_3 0.0))))
          (:then_1
            (Utilities|FlowControl|Delay (Math|Random|RandomFloatinRange 3e+01 5e+01))
            (Audio|Components|Audio|Stop _audiocomponent_3)
            (goto _label_2 Reset)))
        (else
          (Audio|Components|Audio|Stop _audiocomponent_3)
          (goto _label_2 Reset))))
    (:then_2
      ;[1 1 1] Night3
      (if (or (<= _returnvalue 5.3) (>= _returnvalue 20.8))
        (Utilities|FlowControl|Sequence
          (:then_0
            (Utilities|FlowControl|DoOnce false :!label _label_3
              (:Completed
                (Audio|Components|Audio|Play _audiocomponent_4 0.0))))
          (:then_1
            (Utilities|FlowControl|Delay (Math|Random|RandomFloatinRange 3e+01 5e+01))
            (Audio|Components|Audio|Stop _audiocomponent_4)
            (goto _label_3 Reset)))
        (else
          (Audio|Components|Audio|Stop _audiocomponent_4)
          (goto _label_3 Reset))))
    (:then_3
      ;[1 1 1] DayBerg
      (if (and (>= _returnvalue 5.0) (<= _returnvalue 21.0))
        (Utilities|FlowControl|Sequence
          (:then_0
            (Utilities|FlowControl|DoOnce false :!label _label_4
              (:Completed
                (Audio|Components|Audio|Play _audiocomponent_5 0.0))))
          (:then_1
            (Utilities|FlowControl|Delay (Math|Random|RandomFloatinRange 3e+01 5e+01))
            (Audio|Components|Audio|Stop _audiocomponent_5)
            (goto _label_4 Reset)))
        (else
          (Audio|Components|Audio|Stop _audiocomponent_5)
          (goto _label_4 Reset))))
    (:then_4
      ;[1 1 1] Day1
      (if (and (>= _returnvalue 5.0) (<= _returnvalue 21.0))
        (Utilities|FlowControl|Sequence
          (:then_0
            (Utilities|FlowControl|DoOnce false :!label _label_5
              (:Completed
                (Audio|Components|Audio|Play _audiocomponent_6 0.0))))
          (:then_1
            (Utilities|FlowControl|Delay (Math|Random|RandomFloatinRange 3e+01 5e+01))
            (Audio|Components|Audio|Stop _audiocomponent_6)
            (goto _label_5 Reset)))
        (else
          (Audio|Components|Audio|Stop _audiocomponent_6)
          (goto _label_5 Reset))))
    (:then_5
      ;[1 1 1] Day2
      (if (and (>= _returnvalue 5.0) (<= _returnvalue 21.0))
        (Utilities|FlowControl|Sequence
          (:then_0
            (Utilities|FlowControl|DoOnce false :!label _label_6
              (:Completed
                (Audio|Components|Audio|Play _audiocomponent_7 0.0))))
          (:then_1
            (Utilities|FlowControl|Delay (Math|Random|RandomFloatinRange 3e+01 5e+01))
            (Audio|Components|Audio|Stop _audiocomponent_7)
            (goto _label_6 Reset)))
        (else
          (Audio|Components|Audio|Stop _audiocomponent_7)
          (goto _label_6 Reset))))
    (:then_6
      ;[1 1 1] Day3
      (if (and (>= _returnvalue 5.0) (<= _returnvalue 21.0))
        (Utilities|FlowControl|Sequence
          (:then_0
            (Utilities|FlowControl|DoOnce false :!label _label_7
              (:Completed
                (Audio|Components|Audio|Play _audiocomponent_8 0.0))))
          (:then_1
            (Utilities|FlowControl|Delay (Math|Random|RandomFloatinRange 3e+01 5e+01))
            (Audio|Components|Audio|Stop _audiocomponent_8)
            (goto _label_7 Reset)))
        (else
          (Audio|Components|Audio|Stop _audiocomponent_8)
          (goto _label_7 Reset))))
    (:then_7
      ;[1 1 1] Day4
      (if (and (>= _returnvalue 5.0) (<= _returnvalue 21.0))
        (Utilities|FlowControl|Sequence
          (:then_0
            (Utilities|FlowControl|DoOnce false :!label _label_8
              (:Completed
                (Audio|Components|Audio|Play _audiocomponent_9 0.0))))
          (:then_1
            (Utilities|FlowControl|Delay (Math|Random|RandomFloatinRange 3e+01 5e+01))
            (Audio|Components|Audio|Stop _audiocomponent_9)
            (goto _label_8 Reset)))
        (else
          (Audio|Components|Audio|Stop _audiocomponent_9)
          (goto _label_8 Reset))))
    (:then_8
      ;[1 1 1] NightBerg
      (if (or (<= _returnvalue 5.3) (>= _returnvalue 20.8))
        (Utilities|FlowControl|Sequence
          (:then_0
            (Utilities|FlowControl|DoOnce false :!label _label_9
              (:Completed
                (Audio|Components|Audio|Play _audiocomponent 0.0))))
          (:then_1
            (Utilities|FlowControl|Delay (Math|Random|RandomFloatinRange 3e+01 5e+01))
            (Audio|Components|Audio|Stop _audiocomponent)
            (goto _label_9 Reset)))
        (else
          (Audio|Components|Audio|Stop _audiocomponent)
          (goto _label_9 Reset))))))

(fn ConstructionScript)