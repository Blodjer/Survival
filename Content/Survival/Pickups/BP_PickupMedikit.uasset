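; Medikit pickup for the Survival game mode that heals the player who picks it up.
; On pickup it heals the character by the HealHealth amount, then runs the parent pickup logic.
; It is interactable only when the parent allows it and the player is below max health; rendering, verb and name come from the parent.
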(event EventOnPickup
  (params (PlayerCharacter :type Survival%20Player%20Character%20Object%20Reference))
  (Class|SurvivalPlayerCharacter|Heal PlayerCharacter (Variables|Pickup|GetHealHealth))
  (|CallParentFunction PlayerCharacter))

(fn ConstructionScript)

(fn IsRenderedasInteractable
  (bind _returnvalue (|CallParentFunction))
  (return _returnvalue))

(fn IsInteractable
  (params (PlayerCharacter :type Survival%20Player%20Character%20Object%20Reference))
  (bind _returnvalue (|CallParentFunction PlayerCharacter))
  (return (and _returnvalue (< (Variables|/Script/Survival.SurvivalPlayerCharacter|GetHealth PlayerCharacter) (Class|SurvivalPlayerCharacter|GetMaxHealth PlayerCharacter)))))

(fn GetInteractionVerb
  (return (|CallParentFunction)))

(fn GetInteractableName
  (return (|CallParentFunction)))